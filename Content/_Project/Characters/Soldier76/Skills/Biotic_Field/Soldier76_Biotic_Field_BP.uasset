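; Soldier 76's Biotic Field: a thrown or dropped actor that heals characters inside its sphere.
; Sphere overlaps maintain a list of BaseCharacter_BP actors, with no team check.
; A looping timer starts at BeginPlay and adds a set amount of one health type through each listed actor's HealthSystem component.
; On hit, the BioticField component stops physics and collision and the actor moves to the impact point.
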(event OnComponentBeginOverlap(Sphere)
  (params (OverlappedComponent :type Primitive%20Component%20Object%20Reference) (OtherActor :type Actor%20Object%20Reference) (OtherComp :type Primitive%20Component%20Object%20Reference) (OtherBodyIndex :type Integer) (bFromSweep :type Boolean) (SweepResult :type Hit%20Result%20Structure%20%28by%20ref%29))
  (bind _actorsinfield (Variables|Default|GetActorsInField))
  (bind _asbase_character_bp (Utilities|Casting|CastToBaseCharacter_BP OtherActor))
  (if (not (Utilities|Array|ContainsItem _actorsinfield _asbase_character_bp))
    (Utilities|Array|Add _actorsinfield _asbase_character_bp)))

(event OnComponentEndOverlap(Sphere)
  (params (OverlappedComponent :type Primitive%20Component%20Object%20Reference) (OtherActor :type Actor%20Object%20Reference) (OtherComp :type Primitive%20Component%20Object%20Reference) (OtherBodyIndex :type Integer))
  (bind _asbase_character_bp (Utilities|Casting|CastToBaseCharacter_BP OtherActor))
  (Utilities|Array|RemoveItem (Variables|Default|GetActorsInField) _asbase_character_bp))

(event OnComponentHit(BioticField)
  (params (HitComponent :type Primitive%20Component%20Object%20Reference) (OtherActor :type Actor%20Object%20Reference) (OtherComp :type Primitive%20Component%20Object%20Reference) (NormalImpulse :type Vector :default "0, 0, 0") (Hit :type Hit%20Result%20Structure%20%28by%20ref%29))
  (Physics|SetSimulatePhysics HitComponent false)
  (Collision|SetCollisionEnabled HitComponent "NoCollision")
  (Transformation|SetActorLocation (.Location (Collision|BreakHitResult Hit)) false false))

(event Custom|FieldTick
  (for _array_element (Variables|Default|GetActorsInField)
    (Utilities|IsValid (Actor|GetComponentbyClass _array_element "/Game/_Project/CommonSystems/HealthSystem/HealthSystem.HealthSystem_C")
      (:Is%20Valid
        (Default|AddHealthType (Actor|GetComponentbyClass _array_element "/Game/_Project/CommonSystems/HealthSystem/HealthSystem.HealthSystem_C") "NewEnumerator0" (Variables|Default|GetHealAmount))))))

(event EventBeginPlay
  (Utilities|Time|SetTimerbyFunctionName 0 "FieldTick" (Variables|Default|GetTickRate) true))

(fn ConstructionScript)