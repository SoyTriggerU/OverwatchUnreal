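; Soldier 76's ultimate ability, which switches the character to ultimate shooting for a timed window.
; Fire calls the parent, then in one specific ability state switches the owning Soldier76_BP's shooting mode and starts a 7.5-second timer.
; When the timer ends, Finish calls the parent and restores normal shooting.
; Update holds the ultimate charge at zero while the ability is in that same state.
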(event Custom|OnUltimateFinished
  (CallFunction|Finish))

(event EventUpdate
  (params (DeltaTime :type Float%20%28double-precision%29))
  (if (Utilities|Enum|Equal(Enum) (Variables|Default|GetState) "NewEnumerator2")
    (Variables|Default|SetCurrentCharge 0.0)))

(event EventFinish
  (|CallParentFunction)
  (Default|ChangetoNormalShooting (.AsSoldier%2076%20BP (Utilities|Casting|CastToSoldier76_BP (Variables|Default|GetOwningCharacter)))))

(event EventFire
  (|CallParentFunction)
  (if (Utilities|Enum|Equal(Enum) (Variables|Default|GetState) "NewEnumerator2")
    (Default|ChangetoUltimateShooting (.AsSoldier%2076%20BP (Utilities|Casting|CastToSoldier76_BP (Variables|Default|GetOwningCharacter))))
    (Utilities|Time|SetTimerbyEvent (delegate Custom|OnUltimateFinished) 7.5)))