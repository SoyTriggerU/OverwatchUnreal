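; Playable Soldier 76 hero character that sets up health, armor and shield, plus sprint, biotic field and helix rocket skills.
; Enhanced Input drives the skill components and ultimate, with sprinting disabling rockets and the rocket state gating sprint.
; While ultimate shooting is active, Tick sphere-overlaps pawns, picks the one closest to the aim direction by dot product, and smoothly rotates control rotation toward it as an aimbot.
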(event Custom|ChangeToNormalShooting
  (Variables|Default|SetIsUltimateActive false)
  (Variables|Default|SetCurrentLockedTarget 0)
  (Utilities|Array|Clear (Variables|Default|GetTargetCandidates)))

(event Custom|ChangeToUltimateShooting
  (Variables|Default|SetIsUltimateActive true)
  (Variables|Default|SetCurrentLockedTarget 0)
  (Utilities|Array|Clear (Variables|Default|GetTargetCandidates)))

(event Custom|UpdateTargetCandidates
  (bind _outactors (Collision|SphereOverlapActors (Transformation|GetActorLocation) (Variables|Default|GetMaxRange) (Utilities|Array|MakeArray "ObjectTypeQuery3") 0 (Utilities|Array|MakeArray self)))
  (Variables|Default|SetTargetCandidates _outactors))

(event Custom|FindBestTarget
  (Variables|Default|SetBestScore -1.0)
  (Variables|Default|SetCurrentLockedTarget 0)
  (for _array_element (Variables|Default|GetTargetCandidates)
    (bind _output_get (Variables|Default|SetCurrentScore (Math|Vector|DotProduct (Math|Vector|GetForwardVector (Pawn|GetControlRotation :!class /Script/Engine.Pawn)) (Math|Vector|Normalize (- (Transformation|GetActorLocation _array_element) (Transformation|GetWorldLocation (Variables|Default|GetCamera)))))))
    (if (> _output_get (Variables|Default|GetBestScore))
      (Variables|Default|SetBestScore (Variables|Default|GetCurrentScore))
      (bind _output_get_2 (Variables|Default|SetBestTarget _array_element))))
  (Variables|Default|SetCurrentLockedTarget _output_get_2))

(event Input|EnhancedActionEvents|EnhancedInputActionSkill_0
  (params (ActionValue :type Boolean) (ElapsedSeconds :type Float%20%28double-precision%29) (TriggeredSeconds :type Float%20%28double-precision%29) (InputAction :type Input%20Action%20Object%20Reference :default "/Game/_Project/CommonSystems/Input/Skill_0.Skill_0"))
  (bind _soldier76_sprint_skill_bpc (Variables|Default|GetSoldier76_Sprint_Skill_BPC))
  (bind _soldier76_helix_rockets_skill_bpc (Variables|Default|GetSoldier76_Helix_Rockets_Skill_BPC))
  (:Triggered
    (Default|Fire _soldier76_sprint_skill_bpc :!label _label)
    (Default|SetEnabled _soldier76_helix_rockets_skill_bpc false))
  (:Started
    (goto _label))
  (:Canceled
    (Default|Finish _soldier76_sprint_skill_bpc :!label _label_2)
    (Default|SetEnabled _soldier76_helix_rockets_skill_bpc true))
  (:Completed
    (goto _label_2)))

(event Input|EnhancedActionEvents|EnhancedInputActionUltimate
  (params (ActionValue :type Boolean) (ElapsedSeconds :type Float%20%28double-precision%29) (TriggeredSeconds :type Float%20%28double-precision%29) (InputAction :type Input%20Action%20Object%20Reference :default "/Game/_Project/CommonSystems/Input/Ultimate.Ultimate"))
  (:Started
    (Default|Fire (Variables|Default|GetSoldier76_Ultimate_BP))))

(event Input|EnhancedActionEvents|EnhancedInputActionSkill_1
  (params (ActionValue :type Boolean) (ElapsedSeconds :type Float%20%28double-precision%29) (TriggeredSeconds :type Float%20%28double-precision%29) (InputAction :type Input%20Action%20Object%20Reference :default "/Game/_Project/CommonSystems/Input/Skill_1.Skill_1"))
  (bind _soldier76_biotic_field_skill_bpc (Variables|Default|GetSoldier76_Biotic_Field_Skill_BPC))
  (:Started
    (Variables|/Game/_Project/Characters/Soldier76/Skills/Biotic_Field/Soldier76_Biotic_Field_Skill_BPC.Soldier76_Biotic_Field_Skill_BPC_C|SetSpawnPoint _soldier76_biotic_field_skill_bpc (Transformation|GetWorldTransform (Variables|Default|GetBioticFieldSpawnPoint)))
    (Default|Fire _soldier76_biotic_field_skill_bpc)))

(event Input|EnhancedActionEvents|EnhancedInputActionSkill_2
  (params (ActionValue :type Boolean) (ElapsedSeconds :type Float%20%28double-precision%29) (TriggeredSeconds :type Float%20%28double-precision%29) (InputAction :type Input%20Action%20Object%20Reference :default "/Game/_Project/CommonSystems/Input/Skill_2.Skill_2"))
  (bind _soldier76_helix_rockets_skill_bpc (Variables|Default|GetSoldier76_Helix_Rockets_Skill_BPC))
  (:Started
    (Variables|/Game/_Project/Characters/Soldier76/Skills/Helix_Rockets/Soldier76_Helix_Rockets_Skill_BPC.Soldier76_Helix_Rockets_Skill_BPC_C|SetSpawnPoint _soldier76_helix_rockets_skill_bpc (Transformation|GetWorldTransform (Variables|Default|GetHelixRocketsSpawnPoint)))
    (Default|Fire _soldier76_helix_rockets_skill_bpc)))

(event EventBeginPlay
  (bind _soldier76_sprint_skill_bpc (Variables|Default|GetSoldier76_Sprint_Skill_BPC))
  (bind _soldier76_biotic_field_skill_bpc (Variables|Default|GetSoldier76_Biotic_Field_Skill_BPC))
  (bind _soldier76_helix_rockets_skill_bpc (Variables|Default|GetSoldier76_Helix_Rockets_Skill_BPC))
  (|CallParentFunction)
  (Utilities|FlowControl|Sequence
    (:then_0
      (CallFunction|InitializeHealth (Utilities|Struct|MakeHealthData 125.0 125.0 5e+01 5e+01 5e+01 5e+01 0.0 false)))
    (:then_1
      (Default|Initialize _soldier76_sprint_skill_bpc self "L SHIFT")
      (Utilities|Array|Add (Variables|Default|GetSkills) _soldier76_sprint_skill_bpc))
    (:then_2
      (Default|Initialize _soldier76_biotic_field_skill_bpc self "E")
      (Utilities|Array|Add (Variables|Default|GetSkills) _soldier76_biotic_field_skill_bpc))
    (:then_3
      (Default|Initialize _soldier76_helix_rockets_skill_bpc self "RMB")
      (Utilities|Array|Add (Variables|Default|GetSkills) _soldier76_helix_rockets_skill_bpc))))

(event EventTick
  (params (DeltaSeconds :type Float%20%28single-precision%29))
  (bind _currentlockedtarget (Variables|Default|GetCurrentLockedTarget))
  (|CallParentFunction DeltaSeconds)
  (Default|SetEnabled (Variables|Default|GetSoldier76_Sprint_Skill_BPC) (Utilities|Enum|NotEqual(Enum) (Variables|/Game/_Project/CommonSystems/Character_Skills/Character_Skill_BP.Character_Skill_BP_C|GetState (Variables|Default|GetSoldier76_Helix_Rockets_Skill_BPC)) "NewEnumerator1"))
  (if (Variables|Default|GetIsUltimateActive)
    (CallFunction|UpdateTargetCandidates)
    (CallFunction|FindBestTarget)
    (Utilities|IsValid _currentlockedtarget
      (:Is%20Valid
        (bind _asplayer_controller (Utilities|Casting|CastToPlayerController (Pawn|GetController)))
        (Pawn|SetControlRotation _asplayer_controller (Math|Interpolation|RInterpTo (Pawn|GetControlRotation :!class /Script/Engine.Pawn) (Math|Rotator|FindLookatRotation (Transformation|GetWorldLocation (Variables|Default|GetCamera)) (Transformation|GetActorLocation _currentlockedtarget)) (Utilities|Time|GetWorldDeltaSeconds) 15.0))))))

(fn ConstructionScript
  (|CallParentFunction))