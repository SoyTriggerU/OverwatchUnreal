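; Junkrat hero character Blueprint that sets up health, armor and shield and wires inputs to his abilities.
; On BeginPlay it initializes and registers two Concussion Mine skill components and a Steel Trap.
; Skill_0 alternates between the two mine components via a toggle flag, and Skill_2 detonates both.
; Mines and trap fire from a shared spawn point transform, while the Ultimate input fires the ultimate directly.
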(event Input|EnhancedActionEvents|EnhancedInputActionSkill_1
  (params (ActionValue :type Boolean) (ElapsedSeconds :type Float%20%28double-precision%29) (TriggeredSeconds :type Float%20%28double-precision%29) (InputAction :type Input%20Action%20Object%20Reference :default "/Game/_Project/CommonSystems/Input/Skill_1.Skill_1"))
  (bind _steel_trap_skill_bpc (Variables|Default|GetSteel_Trap_Skill_BPC))
  (Variables|/Game/_Project/Characters/Junkrat/Skills/SteelTrap/Steel_Trap_Skill_BPC.Steel_Trap_Skill_BPC_C|SetSpawnPoint _steel_trap_skill_bpc (Transformation|GetWorldTransform (Variables|Default|GetSkillSpawnPoint)))
  (Default|Fire _steel_trap_skill_bpc))

(event Input|EnhancedActionEvents|EnhancedInputActionUltimate
  (params (ActionValue :type Boolean) (ElapsedSeconds :type Float%20%28double-precision%29) (TriggeredSeconds :type Float%20%28double-precision%29) (InputAction :type Input%20Action%20Object%20Reference :default "/Game/_Project/CommonSystems/Input/Ultimate.Ultimate"))
  (:Started
    (Default|Fire (Variables|Default|GetUltimate))))

(event Input|EnhancedActionEvents|EnhancedInputActionSkill_2
  (params (ActionValue :type Boolean) (ElapsedSeconds :type Float%20%28double-precision%29) (TriggeredSeconds :type Float%20%28double-precision%29) (InputAction :type Input%20Action%20Object%20Reference :default "/Game/_Project/CommonSystems/Input/Skill_2.Skill_2"))
  (Default|DetonateMine (Variables|Default|GetConcussion_Mine_Skill_BPC)))

(event Input|EnhancedActionEvents|EnhancedInputActionSkill_0
  (params (ActionValue :type Boolean) (ElapsedSeconds :type Float%20%28double-precision%29) (TriggeredSeconds :type Float%20%28double-precision%29) (InputAction :type Input%20Action%20Object%20Reference :default "/Game/_Project/CommonSystems/Input/Skill_0.Skill_0"))
  (bind _concussion_mine_skill_bpc (Variables|Default|GetConcussion_Mine_Skill_BPC))
  (bind _concussion_mine_skill_bpc1 (Variables|Default|GetConcussion_Mine_Skill_BPC1))
  (:Started
    (if (Variables|Default|GetMineSpawned)
      (Variables|Default|SetMineSpawned false)
      (Variables|/Game/_Project/Characters/Junkrat/Skills/ConcussionMine/Concussion_Mine_Skill_BPC.Concussion_Mine_Skill_BPC_C|SetSpawnPoint _concussion_mine_skill_bpc1 (Transformation|GetWorldTransform (Variables|Default|GetSkillSpawnPoint)))
      (Default|Fire _concussion_mine_skill_bpc1)
      (else
        (Variables|Default|SetMineSpawned true)
        (Variables|/Game/_Project/Characters/Junkrat/Skills/ConcussionMine/Concussion_Mine_Skill_BPC.Concussion_Mine_Skill_BPC_C|SetSpawnPoint _concussion_mine_skill_bpc (Transformation|GetWorldTransform (Variables|Default|GetSkillSpawnPoint)))
        (Default|Fire _concussion_mine_skill_bpc)))))

(event EventBeginPlay
  (bind _concussion_mine_skill_bpc (Variables|Default|GetConcussion_Mine_Skill_BPC))
  (bind _steel_trap_skill_bpc (Variables|Default|GetSteel_Trap_Skill_BPC))
  (bind _concussion_mine_skill_bpc1 (Variables|Default|GetConcussion_Mine_Skill_BPC1))
  (|CallParentFunction)
  (Utilities|FlowControl|Sequence
    (:then_0
      (CallFunction|InitializeHealth (Utilities|Struct|MakeHealthData 125.0 125.0 5e+01 5e+01 5e+01 5e+01 0.0 false)))
    (:then_1
      (Default|Initialize _concussion_mine_skill_bpc self "L SHIFT")
      (Utilities|Array|Add (Variables|Default|GetSkills) _concussion_mine_skill_bpc))
    (:then_2
      (Default|Initialize _concussion_mine_skill_bpc1 self "L SHIFT")
      (Utilities|Array|Add (Variables|Default|GetSkills) _concussion_mine_skill_bpc1))
    (:then_3
      (Default|Initialize _steel_trap_skill_bpc self "E")
      (Utilities|Array|Add (Variables|Default|GetSkills) _steel_trap_skill_bpc))))

(fn ConstructionScript
  (|CallParentFunction))