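; Ashe's ultimate ability Blueprint, which spawns a Bob actor above the owning character.
; Fire works only in one ability state and, on a successful spawn, stores the Bob reference, calls the parent Fire and empties the charge and its UI.
; The ultimate finishes after a fixed delay, or from Update if the Bob reference becomes invalid while in another state, presumably the active one.
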(event EventFinish
  (|CallParentFunction))

(event EventUpdate
  (params (DeltaTime :type Float%20%28double-precision%29))
  (|CallParentFunction DeltaTime)
  (if (Utilities|Enum|Equal(Enum) (Variables|Default|GetState) "NewEnumerator2")
    (Utilities|IsValid (Variables|Default|GetBobRef)
      (:Is%20Not%20Valid
        (CallFunction|Finish)))))

(event EventFire
  (bind _owningcharacter (Variables|Default|GetOwningCharacter))
  (bind _returnvalue (Transformation|GetActorTransform _owningcharacter))
  (if (Utilities|Enum|Equal(Enum) (Variables|Default|GetState) "NewEnumerator1")
    (bind _returnvalue_2 (Game|SpawnActorfromClass "/Game/_Project/Characters/Ashe/Ultimate/Bob_BP.Bob_BP_C" (Math|Transform|MakeTransform (+ (.location _returnvalue) "0.000000,0.000000,200.000000") (.rotation _returnvalue) (.scale _returnvalue)) "DontSpawnIfColliding" "MultiplyWithRoot" 0 0))
    (Utilities|IsValid _returnvalue_2
      (:Is%20Valid
        (Variables|Default|SetBobRef _returnvalue_2)
        (Utilities|FlowControl|Sequence
          (:then_0
            (|CallParentFunction)
            (bind _output_get (Variables|Default|SetCurrentCharge 0.0))
            (Default|SetUltimateAmount (Variables|Default|GetUltimateUI) _output_get))
          (:then_2
            (Utilities|FlowControl|Delay 5.0)
            (CallFunction|Finish)))))))